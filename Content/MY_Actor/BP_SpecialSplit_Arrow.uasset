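; BP_SpecialSplit_Arrow is an arrow actor that splits into three regular arrows.
; Three seconds after BeginPlay it spawns BP_Arrow at two SplitPoint component transforms and at its own transform, then destroys itself.
; A hit on its Box component before then destroys it without splitting.
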(event OnComponentHit(Box)
  (params (HitComponent :type Primitive%20Component%20Object%20Reference) (OtherActor :type Actor%20Object%20Reference) (OtherComp :type Primitive%20Component%20Object%20Reference) (NormalImpulse :type Vector :default "0, 0, 0") (Hit :type Hit%20Result%20Structure%20%28by%20ref%29))
  (Actor|DestroyActor))

(event EventBeginPlay
  (Utilities|FlowControl|Delay 3.0)
  (Game|SpawnActorfromClass "/Game/MY_Actor/BP_Arrow.BP_Arrow_C" (Transformation|GetWorldTransform (Variables|Default|GetSplitPoint1)) "Undefined" 0 0)
  (Game|SpawnActorfromClass "/Game/MY_Actor/BP_Arrow.BP_Arrow_C" (Transformation|GetWorldTransform (Variables|Default|GetSplitPoint2)) "Undefined" 0 0)
  (Game|SpawnActorfromClass "/Game/MY_Actor/BP_Arrow.BP_Arrow_C" (Transformation|GetActorTransform) "Undefined" 0 0)
  (Actor|DestroyActor))

(event Collision|EventActorBeginOverlap
  (params (OtherActor :type Actor%20Object%20Reference)))

(event EventTick
  (params (DeltaSeconds :type Float%20%28single-precision%29)))

(fn ConstructionScript)